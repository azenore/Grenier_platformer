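; BP_FinalDoor is a door actor that moves up when the game instance signals that the cart should appear.
; On BeginPlay it casts to BP_GameInstance and binds OpenFinalDoor to its cart update event, so no Tick is used.
; Each update checks MakeCartAppear: when true it prints a debug string and jumps 500 units above its current height, otherwise it stays in place.
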(event Custom|OpenFinalDoor
  (CallFunction|UpdateTrapDoorFunctiun))

(event EventBeginPlay
  (bind _asbp_game_instance (Utilities|Casting|CastToBP_GameInstance (Game|GetGameInstance)))
  (bind _output_get (Variables|Default|SetAs%20BP%20Game%20Instance _asbp_game_instance))
  (EventDispatchers|BindEventtoUpdateCart _output_get (delegate Custom|OpenFinalDoor)))

(event Collision|EventActorBeginOverlap
  (params (OtherActor :type Actor%20Object%20Reference)))

(event EventTick
  (params (DeltaSeconds :type Float%20%28single-precision%29)))

(fn ConstructionScript)

(fn UpdateTrapDoorFunctiun
  (bind _defaultsceneroot (Variables|Default|GetDefaultSceneRoot))
  (bind _defaultsceneroot_2 (Variables|Default|GetDefaultSceneRoot))
  (bind _returnvalue (Transformation|GetWorldLocation _defaultsceneroot_2))
  (bind _returnvalue_2 (Transformation|GetWorldLocation _defaultsceneroot))
  (if (Variables|/Game/GAME/Blueprints/BP_GameInstance.BP_GameInstance_C|GetMakeCartAppear (Variables|Default|GetAs%20BP%20Game%20Instance))
    (Development|PrintString "OUUUUUUUUUUUUUUUUIIIIIII")
    (Transformation|SetActorLocation (Math|Vector|MakeVector (.x _returnvalue_2) (.y _returnvalue_2) (+ (.z _returnvalue_2) 5e+02)) false false)
    (else
      (Transformation|SetActorLocation (Math|Vector|MakeVector (.x _returnvalue) (.y _returnvalue) (+ (.z _returnvalue) 0.0)) false false))))