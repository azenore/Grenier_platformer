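; BP_DarkCave is an interactable cave entrance that gates travel to the Level5 map behind owning a lantern.
; Interact checks HasLantern on the game instance cached at BeginPlay, then either opens the level or shows the WBP_DarkCave screen widget for a couple of seconds.
; A Box trigger shows the actor's Widget component on overlap and hides it when the overlap ends.
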(event OnComponentBeginOverlap(Box)
  (params (OverlappedComponent :type Primitive%20Component%20Object%20Reference) (OtherActor :type Actor%20Object%20Reference) (OtherComp :type Primitive%20Component%20Object%20Reference) (OtherBodyIndex :type Integer) (bFromSweep :type Boolean) (SweepResult :type Hit%20Result%20Structure%20%28by%20ref%29))
  (Rendering|SetVisibility (Variables|Default|GetWidget) true false))

(event OnComponentEndOverlap(Box)
  (params (OverlappedComponent :type Primitive%20Component%20Object%20Reference) (OtherActor :type Actor%20Object%20Reference) (OtherComp :type Primitive%20Component%20Object%20Reference) (OtherBodyIndex :type Integer))
  (Rendering|SetVisibility (Variables|Default|GetWidget) false false))

(event EventBeginPlay
  (bind _asbp_game_instance (Utilities|Casting|CastToBP_GameInstance (Game|GetGameInstance)))
  (Variables|Default|SetAs%20BP%20Game%20Instance _asbp_game_instance))

(event Collision|EventActorBeginOverlap
  (params (OtherActor :type Actor%20Object%20Reference)))

(event EventTick
  (params (DeltaSeconds :type Float%20%28single-precision%29)))

(event EventInteract
  (if (Variables|/Game/GAME/Blueprints/BP_GameInstance.BP_GameInstance_C|GetHasLantern (Variables|Default|GetAs%20BP%20Game%20Instance))
    (Game|OpenLevel(byObjectReference) "/Game/GAME/Maps/Level5_Map.Level5_Map")
    (else
      (bind _returnvalue (UserInterface|CreateWidget "/Game/GAME/Widgets/WBP_DarkCave.WBP_DarkCave_C"))
      (UserInterface|Viewport|AddtoViewport _returnvalue 0)
      (Utilities|FlowControl|Delay 2.3)
      (Widget|RemovefromParent _returnvalue))))

(fn ConstructionScript)