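; BP_Gates is an interactable gate actor that swings open once by snapping 90 degrees in yaw.
; Activate and deactivate events show and hide its Widget component, with a debug "Hello" print on show.
; Interact runs through a DoOnce, applying the instant rotation and hiding the widget.
; BeginPlay caches the BP_Player pawn, though this graph does not use it afterwards.
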(event EventBeginPlay
  (bind _asbp_player (Utilities|Casting|CastToBP_Player (Game|Player|GetPlayerPawn 0)))
  (Variables|Default|SetAs%20BP%20Player _asbp_player))

(event EventInteract
  (Utilities|FlowControl|DoOnce false
    (:Completed
      (Transformation|SetActorRotation (Math|Rotator|MakeRotator 0.0 0.0 (+ -9e+01 (.yaw (Transformation|GetActorRotation)))))
      (Rendering|SetVisibility (Variables|Default|GetWidget) false false))))

(event EventActivateWidget
  (Rendering|SetVisibility (Variables|Default|GetWidget) true false)
  (Development|PrintString "Hello"))

(event EventUnActivateWidget
  (Rendering|SetVisibility (Variables|Default|GetWidget) false false))

(fn ConstructionScript)