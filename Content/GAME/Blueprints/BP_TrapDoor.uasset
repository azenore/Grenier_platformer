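; Trap door actor that shifts upward when the GameInstance's OpenTrap flag is set.
; It binds to BP_GameInstance's UpdateTrapDoor event on BeginPlay and also runs the update once immediately.
; The update sets the actor's location to the SMWoodPile component's current world position, plus 500 Z when open or zero otherwise.
; No starting position is stored, so the offset is relative to wherever the wood pile currently is.
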(event Custom|Update%20TrapDoor
  (CallFunction|UpdateTrapDoorFunctiun))

(event EventBeginPlay
  (bind _asbp_game_instance (Utilities|Casting|CastToBP_GameInstance (Game|GetGameInstance)))
  (EventDispatchers|BindEventtoUpdateTrapDoor _asbp_game_instance (delegate Custom|Update%20TrapDoor))
  (Variables|Default|SetAs%20BP%20Game%20Instance _asbp_game_instance)
  (CallFunction|UpdateTrapDoorFunctiun))

(event Collision|EventActorBeginOverlap
  (params (OtherActor :type Actor%20Object%20Reference)))

(event EventTick
  (params (DeltaSeconds :type Float%20%28single-precision%29)))

(fn ConstructionScript)

(fn UpdateTrapDoorFunctiun
  (bind _sm_wood_pile (Variables|Default|GetSM_wood_pile))
  (bind _sm_wood_pile_2 (Variables|Default|GetSM_wood_pile))
  (bind _returnvalue (Transformation|GetWorldLocation _sm_wood_pile))
  (bind _returnvalue_2 (Transformation|GetWorldLocation _sm_wood_pile_2))
  (if (Variables|/Game/GAME/Blueprints/BP_GameInstance.BP_GameInstance_C|GetOpenTrap (Variables|Default|GetAs%20BP%20Game%20Instance))
    (Transformation|SetActorLocation (Math|Vector|MakeVector (.x _returnvalue_2) (.y _returnvalue_2) (+ (.z _returnvalue_2) 5e+02)) false false)
    (else
      (Transformation|SetActorLocation (Math|Vector|MakeVector (.x _returnvalue) (.y _returnvalue) (+ (.z _returnvalue) 0.0)) false false))))