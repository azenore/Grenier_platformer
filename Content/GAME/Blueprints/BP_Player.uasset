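; Player Blueprint that handles item collection, object interaction, the main HUD and a menu toggle.
; On overlap, actors with a collectible component go to the collect component, then the HUD refreshes score and coins.
; Overlapped BPI_Interract actors show their message and become the target for the interact input, until overlap ends.
; The menu input uses a FlipFlop to add or remove WBP_MainMenu, without pausing the game.
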(event Input|EnhancedActionEvents|EnhancedInputActionIA_Interact
  (params (ActionValue :type Boolean) (ElapsedSeconds :type Float%20%28double-precision%29) (TriggeredSeconds :type Float%20%28double-precision%29) (InputAction :type Input%20Action%20Object%20Reference :default "/Game/GAME/Blueprints/IA_Interact.IA_Interact"))
  (:Started
    (if (Variables|Default|GetCanInteract)
      (Development|PrintString "Oui")
      (Class|BPIInterract|Interact(Message) (Variables|Default|GetInteractableActor)))))

(event Input|EnhancedActionEvents|EnhancedInputActionIA_Menu
  (params (ActionValue :type Boolean) (ElapsedSeconds :type Float%20%28double-precision%29) (TriggeredSeconds :type Float%20%28double-precision%29) (InputAction :type Input%20Action%20Object%20Reference :default "/Game/GAME/Blueprints/IA_Menu.IA_Menu"))
  ;[1 1 1] Open pause menu
  (:Started
    (Utilities|FlowControl|FlipFlop
      (:A
        (bind _returnvalue (UserInterface|CreateWidget "/Game/GAME/Widgets/WBP_MainMenu.WBP_MainMenu_C"))
        (UserInterface|Viewport|AddtoViewport _returnvalue 0))
      (:B
        (Widget|RemovefromParent _returnvalue)))))

(event EventBeginPlay
  (|CallParentFunction)
  (bind _returnvalue (UserInterface|CreateWidget "/Game/GAME/Blueprints/BPW_MainHud.BPW_MainHud_C"))
  (bind _output_get (Variables|Default|SetWidget _returnvalue))
  (UserInterface|Viewport|AddtoViewport _output_get 0))

(event Collision|EventActorEndOverlap
  (params (OtherActor :type Actor%20Object%20Reference))
  (bind _interactableactor (Variables|Default|GetInteractableActor))
  (if (== OtherActor _interactableactor)
    (Variables|Default|SetCanInteract false)
    (Class|BPIInterract|UnActivateWidget(Message) _interactableactor)))

(event EventTick
  (params (DeltaSeconds :type Float%20%28single-precision%29)))

(event Collision|EventActorBeginOverlap
  (params (OtherActor :type Actor%20Object%20Reference))
  (Utilities|FlowControl|Sequence
    (:then_0
      (CallFunction|CollectObject OtherActor))
    (:then_1
      (if (Utilities|DoesObjectImplementInterface OtherActor "/Game/GAME/Blueprints/BPI_Interract.BPI_Interract_C")
        (Variables|Default|SetCanInteract true)
        (bind _output_get (Variables|Default|SetInteractableActor OtherActor))
        (Class|BPIInterract|ActivateWidget(Message) _output_get)))))

(fn ConstructionScript
  (|CallParentFunction))

(fn CollectObject
  (params (NewParam :type Actor%20Object%20Reference))
  (bind _returnvalue (Actor|GetComponentbyClass NewParam "/Game/GAME/Blueprints/BPC_CollectibleComponent.BPC_CollectibleComponent_C"))
  (bind _widget (Variables|Default|GetWidget))
  (Utilities|IsValid _returnvalue
    (:Is%20Valid
      (Default|Collect (Variables|Default|GetBPC_CollectComponent) _returnvalue)
      (Default|UpdateScore _widget)
      (Default|UpdateCoins _widget))))