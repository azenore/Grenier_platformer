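; BP_HouseDoor is a house door actor that serves as the entrance to Level 3.
; On BeginPlay it reads HouseDoorOpen from BP_GameInstance and, if set, swings itself open by a yaw offset and allows Level 3 access.
; Its Interact event loads Level3_Map only when that access is granted.
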(event EventBeginPlay
  (bind _asbp_game_instance (Utilities|Casting|CastToBP_GameInstance (Game|GetGameInstance)))
  (if (Variables|/Game/GAME/Blueprints/BP_GameInstance.BP_GameInstance_C|GetHouseDoorOpen _asbp_game_instance)
    (Transformation|SetActorRotation (Math|Rotator|MakeRotator 0.0 0.0 (+ (.yaw (Transformation|GetActorRotation)) -9e+01)))
    (Variables|Default|SetCanAccessLevel3 true)
    (else
      (Transformation|SetActorRotation (Math|Rotator|MakeRotator 0.0 0.0 (+ (.yaw (Transformation|GetActorRotation)) 0.0))))))

(event Collision|EventActorBeginOverlap
  (params (OtherActor :type Actor%20Object%20Reference)))

(event EventTick
  (params (DeltaSeconds :type Float%20%28single-precision%29)))

(event EventInteract
  (if (Variables|Default|GetCanAccessLevel3)
    (Game|OpenLevel(byObjectReference) "/Game/GAME/Maps/level3_Map.level3_Map")))

(fn ConstructionScript)